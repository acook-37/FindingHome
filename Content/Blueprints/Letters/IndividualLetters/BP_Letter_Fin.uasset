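; BP_Letter_Fin is a letter pickup that the first-person character takes by pressing E while it is selected.
; Tick enables player input on the actor only while it is selected and not yet held.
; Pressing E toggles the player's letter hold, sets the held flag, hides both cube meshes and toggles selectability.
; BeginPlay caches the character reference, and the IsSelected function always returns false.
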(event EventTick
  (params (DeltaSeconds :type Float%20%28single-precision%29))
  (if (Variables|Default|GetHoldToggled?)
    (Input|DisableInput (Game|GetPlayerController 0))
    (elif (Variables|Default|GetSelected?)
      (Input|EnableInput (Game|GetPlayerController 0))
      (else
        (Input|DisableInput (Game|GetPlayerController 0))))))

(event EventBeginPlay
  (bind _returnvalue (Actor|GetActorOfClass "/Game/FirstPerson/Blueprints/BP_FirstPersonCharacter.BP_FirstPersonCharacter_C"))
  (Variables|Default|SetPlayerChar _returnvalue))

(event Input|KeyboardEvents|E
  (params (Key :type Key%20Structure :default "None"))
  (:Pressed
    (Default|ToggleLetterHold (Variables|Default|GetPlayerChar))
    (Variables|Default|SetHoldToggled? true)
    (Rendering|SetVisibility (Variables|Default|GetCube_0) false false)
    (Rendering|SetVisibility (Variables|Default|GetCube) false false)
    (CallFunction|ToggleSelectable)))

(fn ConstructionScript
  (|CallParentFunction))

(fn IsSelected?
  (return false))