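; BP_Typewriter is a typewriter actor that spawns a BP_Letter_F1 actor when the player presses E while it is selected.
; Tick polls the Selected flag every frame to enable or disable input from player controller 0, so E only reaches the selected typewriter.
; The letter spawns at the LetterSpawn transform, and HasSpawned limits it to a single spawn.
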(event EventTick
  (params (DeltaSeconds :type Float%20%28single-precision%29))
  (if (Variables|Default|GetSelected?)
    (Input|EnableInput (Game|GetPlayerController 0))
    (else
      (Input|DisableInput (Game|GetPlayerController 0)))))

(event Input|KeyboardEvents|E
  (params (Key :type Key%20Structure :default "None"))
  (:Pressed
    (if (not (Variables|Default|GetHasSpawned?))
      (Game|SpawnActorfromClass "/Game/Blueprints/Letters/IndividualLetters/BP_Letter_F1.BP_Letter_F1_C" (Variables|Default|GetLetterSpawn) "Undefined" 0 0)
      (Variables|Default|SetHasSpawned? true))))

(fn ConstructionScript
  (|CallParentFunction))