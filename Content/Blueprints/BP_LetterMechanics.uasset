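; BP_LetterMechanics handles opening a letter popup when the player toggles a letter.
; ToggleLetter prints a debug string, then, if InLetter is false and IsFacing is true, creates BP_Widget, stores it as LetterPopup and adds it to the viewport.
; An unconnected node would copy IsLooking from InteractableBox into IsFacing but never runs, and nothing here sets InLetter or closes the popup.
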(event Custom|ToggleLetter
  (Development|PrintString "Toggling")
  (if (not (Variables|Default|GetInLetter))
    (if (Variables|Default|GetIsFacing)
      (bind _returnvalue (UserInterface|CreateWidget "/Game/Blueprints/BP_Widget.BP_Widget_C"))
      (bind _output_get (Variables|Default|SetLetterPopup _returnvalue))
      (UserInterface|Viewport|AddtoViewport _output_get 0))))