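; Endgame typewriter that, on E once the player's ReadCount is exactly nine, runs Read1stLetter and unlocks the generator door; otherwise it briefly shows a not-ready widget.
; Tick caches the open letter widgets and enables input only while Selected.
; Read1stLetter spawns the final letter actor once and toggles a range-checked reading widget, freezing movement and look.
; Near-identical second and third letter functions exist but are never called here.
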(event EventBeginPlay
  (bind _returnvalue (Actor|GetActorOfClass "/Game/FirstPerson/Blueprints/BP_FirstPersonCharacter.BP_FirstPersonCharacter_C"))
  (Variables|Default|SetPlayer%20Char _returnvalue)
  (bind _returnvalue_2 (Actor|GetActorOfClass "/Game/Blueprints/BP_genDoor.BP_genDoor_C"))
  (Variables|Default|SetGen%20Door _returnvalue_2))

(event EventTick
  (params (DeltaSeconds :type Float%20%28single-precision%29))
  (bind _foundwidgets (Widget|GetAllWidgetsOfClass "/Game/Blueprints/Letters/IndividualLetters/Widgets/BPW_Final.BPW_Final_C" true))
  (Variables|Default|SetFoundBP1 _foundwidgets)
  (bind _foundwidgets_2 (Widget|GetAllWidgetsOfClass "/Game/Blueprints/Letters/IndividualLetters/Widgets/BPW_F2P1.BPW_F2P1_C" true))
  (Variables|Default|SetFoundBP2 _foundwidgets_2)
  (bind _foundwidgets_3 (Widget|GetAllWidgetsOfClass "/Game/Blueprints/Letters/IndividualLetters/Widgets/BPW_F3P1.BPW_F3P1_C" true))
  (Variables|Default|SetFoundBP3 _foundwidgets_3)
  (if (Variables|Default|GetSelected?)
    (Input|EnableInput (Game|GetPlayerController 0))
    (else
      (Input|DisableInput (Game|GetPlayerController 0)))))

(event Input|KeyboardEvents|E
  (params (Key :type Key%20Structure :default "None"))
  (:Pressed
    (if (== (Variables|/Game/FirstPerson/Blueprints/BP_FirstPersonCharacter.BP_FirstPersonCharacter_C|GetReadCount (Variables|Default|GetPlayer%20Char)) 9)
      (if true
        (CallFunction|Read1stLetter)
        (Variables|/Game/Blueprints/BP_genDoor.BP_genDoor_C|SetLocked? (Variables|Default|GetGen%20Door) false))
      (elif (Variables|Default|GetDoPrinting?)
        (bind _returnvalue (UserInterface|CreateWidget "/Game/Blueprints/Widgets/BPW_NotReady.BPW_NotReady_C"))
        (UserInterface|Viewport|AddtoViewport _returnvalue 0)
        (Variables|Default|SetDoPrinting? false)
        (Utilities|FlowControl|Delay (Variables|Default|GetDelay))
        (Widget|RemovefromParent _returnvalue)
        (Variables|Default|SetDoPrinting? true)))))

(event Input|MouseEvents|LeftMouseButton
  (params (Key :type Key%20Structure :default "None"))
  (:Pressed
    (Development|PrintString "Left Click")))

(fn ConstructionScript
  (|CallParentFunction))

(fn Read1stLetter
  (bind _returnvalue (Game|GetPlayerController 0))
  (bind _returnvalue_2 (Game|GetPlayerController 0))
  (if (Variables|Default|GetHasSpawned?)
    _
    (else
      (Game|SpawnActorfromClass "/Game/Blueprints/Letters/IndividualLetters/BP_Letter_Fin.BP_Letter_Fin_C" (Variables|Default|GetLetterSpawn) "Undefined" 0 0)
      (Variables|Default|SetHasSpawned? true)))
  (if (Variables|Default|GetSelected?)
    (Development|PrintString "Letter is being looked at!")
    (else
      (Development|PrintString "Letter not being looked at!")))
  (if (Variables|Default|GetReading%20Letter)
    (Variables|Default|SetReading%20Letter false)
    (Input|SetIgnoreMoveInput _returnvalue false)
    (Input|SetIgnoreLookInput _returnvalue false)
    (Widget|RemovefromParent (Variables|Default|GetFoundBP1))
    (Utilities|IsValid (Variables|Default|GetLetter%202)
      (:Is%20Valid
        (Widget|RemovefromParent (Variables|Default|GetFoundBP2))))
    (elif (Variables|Default|GetSelected?)
      (bind _output_get (Variables|Default|SetPlayer%20Distance (Transformation|GetDistanceTo (Game|GetPlayerCharacter 0) self)))
      (if (<= _output_get 4.5e+02)
        (bind _returnvalue_3 (UserInterface|CreateWidget "/Game/Blueprints/Letters/IndividualLetters/Widgets/BPW_Final.BPW_Final_C"))
        (Variables|Default|SetLetter%201 _returnvalue_3)
        (UserInterface|Viewport|AddtoViewport _returnvalue_3 0)
        (Variables|Default|SetReading%20Letter true)
        (Variables|/Script/Engine.MovementComponent|SetVelocity (Variables|/Script/Engine.Character|GetCharacterMovement (Game|GetPlayerCharacter 0)) "0, 0, 0")
        (Input|SetIgnoreMoveInput _returnvalue_2 true)
        (Input|SetIgnoreLookInput _returnvalue_2 true)
        (else
          (Development|PrintString "Too far away"))))))

(fn Read2ndLetter
  (bind _returnvalue (Game|GetPlayerController 0))
  (bind _returnvalue_2 (Game|GetPlayerController 0))
  (if (Variables|Default|GetHasSpawned?)
    _
    (else
      (Game|SpawnActorfromClass "/Game/Blueprints/Letters/IndividualLetters/BP_Letter_Fin.BP_Letter_Fin_C" (Variables|Default|GetLetterSpawn) "Undefined" 0 0)
      (Variables|Default|SetHasSpawned? true)))
  (if (Variables|Default|GetSelected?)
    (Development|PrintString "Letter is being looked at!")
    (else
      (Development|PrintString "Letter not being looked at!")))
  (if (Variables|Default|GetReading%20Letter)
    (Variables|Default|SetReading%20Letter false)
    (Input|SetIgnoreMoveInput _returnvalue false)
    (Input|SetIgnoreLookInput _returnvalue false)
    (Widget|RemovefromParent (Variables|Default|GetFoundBP1))
    (Utilities|IsValid (Variables|Default|GetLetter%202)
      (:Is%20Valid
        (Widget|RemovefromParent (Variables|Default|GetFoundBP2))))
    (elif (Variables|Default|GetSelected?)
      (bind _output_get (Variables|Default|SetPlayer%20Distance (Transformation|GetDistanceTo (Game|GetPlayerCharacter 0) self)))
      (if (<= _output_get 4.5e+02)
        (bind _returnvalue_3 (UserInterface|CreateWidget "/Game/Blueprints/Letters/IndividualLetters/Widgets/BPW_F2P1.BPW_F2P1_C"))
        (Variables|Default|SetLetter%202 _returnvalue_3)
        (UserInterface|Viewport|AddtoViewport _returnvalue_3 0)
        (Variables|Default|SetReading%20Letter true)
        (Variables|/Script/Engine.MovementComponent|SetVelocity (Variables|/Script/Engine.Character|GetCharacterMovement (Game|GetPlayerCharacter 0)) "0, 0, 0")
        (Input|SetIgnoreMoveInput _returnvalue_2 true)
        (Input|SetIgnoreLookInput _returnvalue_2 true)
        (else
          (Development|PrintString "Too far away"))))))

(fn Read3rdLetter
  (bind _returnvalue (Game|GetPlayerController 0))
  (bind _returnvalue_2 (Game|GetPlayerController 0))
  (if (Variables|Default|GetHasSpawned?)
    _
    (else
      (Game|SpawnActorfromClass "/Game/Blueprints/Letters/IndividualLetters/BP_Letter_Fin.BP_Letter_Fin_C" (Variables|Default|GetLetterSpawn) "Undefined" 0 0)
      (Variables|Default|SetHasSpawned? true)))
  (if (Variables|Default|GetSelected?)
    (Development|PrintString "Letter is being looked at!")
    (else
      (Development|PrintString "Letter not being looked at!")))
  (if (Variables|Default|GetReading%20Letter)
    (Variables|Default|SetReading%20Letter false)
    (Input|SetIgnoreMoveInput _returnvalue false)
    (Input|SetIgnoreLookInput _returnvalue false)
    (Widget|RemovefromParent (Variables|Default|GetFoundBP3))
    (Utilities|IsValid (Variables|Default|GetLetter%202)
      (:Is%20Valid
        (Widget|RemovefromParent (Variables|Default|GetFoundBP2))))
    (elif (Variables|Default|GetSelected?)
      (bind _output_get (Variables|Default|SetPlayer%20Distance (Transformation|GetDistanceTo (Game|GetPlayerCharacter 0) self)))
      (if (<= _output_get 4.5e+02)
        (bind _returnvalue_3 (UserInterface|CreateWidget "/Game/Blueprints/Letters/IndividualLetters/Widgets/BPW_F3P1.BPW_F3P1_C"))
        (Variables|Default|SetLetter%203 _returnvalue_3)
        (UserInterface|Viewport|AddtoViewport _returnvalue_3 0)
        (Variables|Default|SetReading%20Letter true)
        (Variables|/Script/Engine.MovementComponent|SetVelocity (Variables|/Script/Engine.Character|GetCharacterMovement (Game|GetPlayerCharacter 0)) "0, 0, 0")
        (Input|SetIgnoreMoveInput _returnvalue_2 true)
        (Input|SetIgnoreLookInput _returnvalue_2 true)
        (else
          (Development|PrintString "Too far away"))))))