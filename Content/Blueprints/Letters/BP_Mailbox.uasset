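; BP_Mailbox is an interactable mailbox where the first-person character deposits a held letter with the E key.
; Tick enables or disables the actor's input from the Selected flag, which this graph only reads.
; E toggles off the hold and increments the letter count on the character cached at BeginPlay.
; Without a letter, it shows a BPW_NoLetter widget for a second, guarded by DoPrinting against stacking.
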(event EventTick
  (params (DeltaSeconds :type Float%20%28single-precision%29))
  (if (Variables|Default|GetSelected?)
    (Input|EnableInput (Game|GetPlayerController 0))
    (else
      (Input|DisableInput (Game|GetPlayerController 0)))))

(event EventBeginPlay
  (bind _returnvalue (Actor|GetActorOfClass "/Game/FirstPerson/Blueprints/BP_FirstPersonCharacter.BP_FirstPersonCharacter_C"))
  (Variables|Default|SetPlayer%20Char _returnvalue))

(event Input|KeyboardEvents|E
  (params (Key :type Key%20Structure :default "None"))
  (bind _player_char (Variables|Default|GetPlayer%20Char))
  (:Pressed
    (if (Variables|/Game/FirstPerson/Blueprints/BP_FirstPersonCharacter.BP_FirstPersonCharacter_C|GetHoldingLetter (Variables|Default|GetPlayer%20Char))
      (Development|PrintString "Found Letter")
      (Default|ToggleLetterHold _player_char)
      (Default|IncreaseLetterCount _player_char)
      (else
        (Development|PrintString "Didn't FInd Letter")
        (if (Variables|Default|GetDoPrinting?)
          (bind _returnvalue (UserInterface|CreateWidget "/Game/Blueprints/Widgets/BPW_NoLetter.BPW_NoLetter_C"))
          (bind _output_get (Variables|Default|SetFailText _returnvalue))
          (UserInterface|Viewport|AddtoViewport _returnvalue 0)
          (Variables|Default|SetDoPrinting? false)
          (Utilities|FlowControl|Delay 1.0)
          (Widget|RemovefromParent _output_get)
          (Variables|Default|SetDoPrinting? true))))))

(fn ConstructionScript
  (|CallParentFunction))