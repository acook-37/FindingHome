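; BP_EndTrigger is a trigger actor that ends the game when the first-person player overlaps it.
; On overlap with BP_FirstPersonCharacter it zeroes the character's velocity and has the player controller ignore move and look input.
; It then creates the BPW_EndScreen widget and adds it to the viewport.
; BeginPlay also stores a reference to the character, though the overlap logic does not use it.
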(event EventBeginPlay
  (bind _returnvalue (Actor|GetActorOfClass "/Game/FirstPerson/Blueprints/BP_FirstPersonCharacter.BP_FirstPersonCharacter_C"))
  (Variables|Default|SetPlayerChar _returnvalue))

(event Collision|EventActorBeginOverlap
  (params (OtherActor :type Actor%20Object%20Reference))
  (bind _returnvalue (Game|GetPlayerController 0))
  (Utilities|Casting|CastToBP_FirstPersonCharacter OtherActor)
  (Variables|/Script/Engine.MovementComponent|SetVelocity (Variables|/Script/Engine.Character|GetCharacterMovement (Game|GetPlayerCharacter 0)) "0, 0, 0")
  (Input|SetIgnoreMoveInput _returnvalue true)
  (Input|SetIgnoreLookInput _returnvalue true)
  (bind _returnvalue_2 (UserInterface|CreateWidget "/Game/Blueprints/Widgets/BPW_EndScreen.BPW_EndScreen_C"))
  (UserInterface|Viewport|AddtoViewport _returnvalue_2 0))

(event EventTick
  (params (DeltaSeconds :type Float%20%28single-precision%29)))

(fn ConstructionScript)