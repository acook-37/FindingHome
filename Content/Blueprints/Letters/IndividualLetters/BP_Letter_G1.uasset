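; BP_Letter_G1 is a readable two-page letter prop that the player opens with E when it is Selected and within range.
; Opening swaps the mesh, shows the page-one widget and freezes player movement and look; left click adds page two.
; E removes the pages using widget lists refreshed every Tick, but only restores control once page two has been created.
; Debug prints trace input, and IsSelected always returns false.
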(event EventTick
  (params (DeltaSeconds :type Float%20%28single-precision%29))
  (bind _foundwidgets (Widget|GetAllWidgetsOfClass "/Game/Blueprints/Letters/IndividualLetters/Widgets/BPW_G1P1.BPW_G1P1_C" true))
  (Variables|Default|SetFoundBP1 _foundwidgets)
  (bind _foundwidgets_2 (Widget|GetAllWidgetsOfClass "/Game/Blueprints/Letters/IndividualLetters/Widgets/BPW_G1P2.BPW_G1P2_C" true))
  (Variables|Default|SetFoundBP2 _foundwidgets_2))

(event EventBeginPlay
  (Input|EnableInput (Game|GetPlayerController 0)))

(event Input|KeyboardEvents|E
  (params (Key :type Key%20Structure :default "None"))
  (bind _returnvalue (Game|GetPlayerController 0))
  (bind _returnvalue_2 (Game|GetPlayerController 0))
  (:Pressed
    (Development|PrintString "E key press")
    (if (Variables|Default|GetSelected?)
      (Development|PrintString "Letter is being looked at!")
      (else
        (Development|PrintString "Letter not being looked at!")))
    (if (Variables|Default|GetReadingLetter)
      (Widget|RemovefromParent (Variables|Default|GetFoundBP1))
      (Utilities|IsValid (Variables|Default|GetLetterPage2)
        (:Is%20Valid
          (Widget|RemovefromParent (Variables|Default|GetFoundBP2))
          (Variables|Default|SetReadingLetter false)
          (Input|SetIgnoreMoveInput _returnvalue false)
          (Input|SetIgnoreLookInput _returnvalue false)))
      (elif (Variables|Default|GetSelected?)
        (bind _output_get (Variables|Default|SetPlayerDistance (Transformation|GetDistanceTo (Game|GetPlayerCharacter 0) self)))
        (if (<= _output_get 4.5e+02)
          (bind _returnvalue_3 (UserInterface|CreateWidget "/Game/Blueprints/Letters/IndividualLetters/Widgets/BPW_G1P1.BPW_G1P1_C"))
          (Variables|Default|SetLetterPage1 _returnvalue_3)
          (UserInterface|Viewport|AddtoViewport _returnvalue_3 0)
          (Variables|Default|SetReadingLetter true)
          (Components|StaticMesh|SetStaticMesh (Variables|Default|GetCube) (Variables|Default|GetOpenLetter))
          (Variables|/Script/Engine.MovementComponent|SetVelocity (Variables|/Script/Engine.Character|GetCharacterMovement (Game|GetPlayerCharacter 0)) "0, 0, 0")
          (Input|SetIgnoreMoveInput _returnvalue_2 true)
          (Input|SetIgnoreLookInput _returnvalue_2 true)
          (else
            (Development|PrintString "Too far away")))))))

(event Input|MouseEvents|LeftMouseButton
  (params (Key :type Key%20Structure :default "None"))
  (:Pressed
    (Development|PrintString "Left Click")
    (if (Variables|Default|GetReadingLetter)
      (Development|PrintString "Are Reading!")
      (bind _returnvalue (UserInterface|CreateWidget "/Game/Blueprints/Letters/IndividualLetters/Widgets/BPW_G1P2.BPW_G1P2_C"))
      (Variables|Default|SetLetterPage2 _returnvalue)
      (UserInterface|Viewport|AddtoViewport _returnvalue 0)
      (else
        (Development|PrintString "Not Reading!")))))

(fn ConstructionScript
  (|CallParentFunction))

(fn IsSelected?
  (return false))